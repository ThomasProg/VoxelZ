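; AC_Attack is an attack component that deals melee-agnostic damage to a focused target and reports its remaining health.
; Attack subtracts PhysicalStrength directly from the target's AC_Life HP, returning a validity flag with current and max HP.
; A killed PAWNX quits the game, while other targets are destroyed.
; Survivors get their health bar updated through casts to the MyNPC widget or PAWNX UI.
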(fn `Attack`
  (returns (isValid :type Boolean) (`HP Actu` :type "Float (double-precision)") (`HP Max` :type "Float (double-precision)"))
  (bind _focused_target (`self.Focused target`))
  (bind _returnvalue (`Actor.GetComponentByClass` _focused_target "/Game/Assets/AI/NPCs/AC_Life.AC_Life_C"))
  (bind _hp_max (`/Game/Assets/AI/NPCs/AC_Life.HP Max` _returnvalue))
  (bind _hp_actu (`/Game/Assets/AI/NPCs/AC_Life.HP Actu` _returnvalue))
  (bind _returnvalue_2 (/ _hp_actu _hp_max))
  ;[1 1 1] Is Valid
  (`/Engine/EditorBlueprintResources/StandardMacros.IsValid` _focused_target
    (:`Is Valid`
      (`/Engine/EditorBlueprintResources/StandardMacros.IsValid` _returnvalue
        (:`Is Valid`
          ;[1 1 1] Deal Damages
          (bind _output_get (set `/Game/Assets/AI/NPCs/AC_Life.HP Actu` (- _hp_actu (`self.Physical Strength`)) _returnvalue))
          (if (<= _output_get 0.0)
            ;[1 1 1] Kill Target
            (cast `/Game/Assets/PAWNX` _focused_target
              (:`then`
                (`KismetSystemLibrary.QuitGame` null "Quit"))
              (:`CastFailed`
                (`Actor.K2_DestroyActor` _focused_target)))
            (return false 0.0 0.0)
            (else
              (bind _asmy_npc (cast `/Game/Assets/AI/NPCs/Entities/MyNPC` _focused_target)
                (:`then`
                  (bind _aslife_bar (cast `/Game/Assets/UI/LifeBar` (`WidgetComponent.GetUserWidgetObject` (`/Game/Assets/AI/NPCs/Entities/MyNPC.Widget` _asmy_npc))))
                  (`ProgressBar.SetPercent` (`/Game/Assets/UI/LifeBar.ProgressBar_29` _aslife_bar) _returnvalue_2))
                (:`CastFailed`
                  (bind _aspawnx (cast `/Game/Assets/PAWNX` _focused_target))
                  (bind _ui_ref (`/Game/Assets/PAWNX.UI ref` _aspawnx))
                  (`/Engine/EditorBlueprintResources/StandardMacros.IsValid` _ui_ref
                    (:`Is Valid`
                      (`ProgressBar.SetPercent` (`/Game/Assets/UI/UI_main.ProgressBar_life` _ui_ref) _returnvalue_2)))))
              (return true _hp_actu _hp_max))))
        (:`Is Not Valid`
          _)))
    (:`Is Not Valid`
      _))
  (return false 0.0 0.0))