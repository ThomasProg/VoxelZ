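; Vehicle reference-frame actor that carries a set of voxel chunks, moving and rotating them as one body.
; Movement and rotation events update the actor, then the chunks in the PlayerController's hard-coded ChunksManagement slot 1, rebuilding positions from chunk coordinates on set or rotate.
; SpawnVoxel returns an origin-adjusted, actor-aligned transform plus voxel sizing.
; BeginPlay snaps Cube to the player pawn after a short delay; collision-ignore and debug chains are unwired.
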(event `self.ReceiveBeginPlay`
  (bind _returnvalue (`GameplayStatics.GetPlayerPawn` 0))
  (`KismetSystemLibrary.Delay` 0.2)
  (`/Engine/EditorBlueprintResources/StandardMacros.IsValid` _returnvalue
    (:`Is Valid`
      (`SceneComponent.K2_SetWorldLocation` (`self.Cube`) (`self.K2_GetActorLocation` _returnvalue) false false))))

(event `AddMovement`
  (params (NewParam :type "Vector Structure"))
  (`self.K2_AddActorWorldOffset` NewParam true true)
  (bind _aspc (cast `/Game/Assets/PC` (`GameplayStatics.GetPlayerController` 0)))
  (bind _chunksmanagement (`MyPlayerController.chunksManagement` _aspc))
  (if (`KismetArrayLibrary.Array_IsValidIndex` _chunksmanagement 1)
    (bind (_output_lastplayerchunk _output_chunksref) (break `S_EachReferencialChunk_Management` (`|GetArrayItem` _chunksmanagement 1)))
    (for _array_element _output_chunksref
      (`self.K2_AddActorWorldOffset` _array_element NewParam false false))))

(event `SetLocation`
  (params (NewParam :type "Vector Structure"))
  (`self.K2_SetActorLocation` NewParam true true)
  (bind _aspc (cast `/Game/Assets/PC` (`GameplayStatics.GetPlayerController` 0)))
  (bind _chunksmanagement (`MyPlayerController.chunksManagement` _aspc))
  (if (`KismetArrayLibrary.Array_IsValidIndex` _chunksmanagement 1)
    (bind (_output_lastplayerchunk _output_chunksref) (break `S_EachReferencialChunk_Management` (`|GetArrayItem` _chunksmanagement 1)))
    (for _array_element _output_chunksref
      (`self.K2_SetActorLocation` _array_element (+ (`Utilities.FIntVector_times_FVector` (`VoxelActor.ChunkCoordonates` _array_element) (`Utilities.FIntVector_times_FVector` (`VoxelActor.chunkLineElements` _array_element) (`VoxelActor.FvoxelSize` _array_element))) NewParam) false false))))

(event `self.ReceiveTick`
  (params (DeltaSeconds :type "Float (single-precision)")))

(event `AddRotation`
  (params (NewParam :type "Rotator Structure"))
  (bind _aspc (cast `/Game/Assets/PC` (`GameplayStatics.GetPlayerController` 0)))
  (`self.K2_AddActorWorldRotation` NewParam true true)
  (bind (_output_lastplayerchunk _output_chunksref) (break `S_EachReferencialChunk_Management` (`|GetArrayItem` (`MyPlayerController.chunksManagement` _aspc) 1)))
  (for _array_element _output_chunksref
    (`self.K2_AddActorWorldRotation` _array_element NewParam false false)
    (bind (_chunkcoordonates_x _chunkcoordonates_y _chunkcoordonates_z) (break `IntVector` (`VoxelActor.ChunkCoordonates` _array_element)))
    (`self.K2_SetActorLocation` _array_element (+ (* (`Utilities.FIntVector_times_FVector` (`VoxelActor.chunkLineElements` _array_element) (`VoxelActor.FvoxelSize` _array_element)) (+ (* (`self.GetActorForwardVector`) _chunkcoordonates_x) (* (`self.GetActorRightVector`) _chunkcoordonates_y) (* (`self.GetActorUpVector`) _chunkcoordonates_z))) (`self.K2_GetActorLocation`)) false false)))

(event `SetRotation`
  (params (NewParam :type "Rotator Structure"))
  (bind _aspc (cast `/Game/Assets/PC` (`GameplayStatics.GetPlayerController` 0)))
  (`self.K2_SetActorRotation` NewParam true)
  (bind (_output_lastplayerchunk _output_chunksref) (break `S_EachReferencialChunk_Management` (`|GetArrayItem` (`MyPlayerController.chunksManagement` _aspc) 1)))
  (for _array_element _output_chunksref
    (`self.K2_SetActorRotation` _array_element NewParam false)
    (bind (_chunkcoordonates_x _chunkcoordonates_y _chunkcoordonates_z) (break `IntVector` (`VoxelActor.ChunkCoordonates` _array_element)))
    (`self.K2_SetActorLocation` _array_element (+ (* (`Utilities.FIntVector_times_FVector` (`VoxelActor.chunkLineElements` _array_element) (`VoxelActor.FvoxelSize` _array_element)) (+ (* (`self.GetActorForwardVector`) _chunkcoordonates_x) (* (`self.GetActorRightVector`) _chunkcoordonates_y) (* (`self.GetActorUpVector`) _chunkcoordonates_z))) (`self.K2_GetActorLocation`)) false false)))

(fn `SpawnVoxel`
  (params (location :type "Vector Structure"))
  (returns (transform :type "Transform Structure") (FVoxelSize :type "Vector Structure") (FChunkLineElements :type "IntVector Structure"))
  (bind (_returnvalue_x _returnvalue_y _returnvalue_z) (break `IntVector` (`GameplayStatics.GetWorldOriginLocation`)))
  (return (`KismetMathLibrary.MakeTransform` (- location (`KismetMathLibrary.MakeVector` (`KismetMathLibrary.Conv_IntToDouble` _returnvalue_x) (`KismetMathLibrary.Conv_IntToDouble` _returnvalue_y) (`KismetMathLibrary.Conv_IntToDouble` _returnvalue_z))) (`self.K2_GetActorRotation`)) (* (`KismetMathLibrary.MakeVector` 1.0 1.0 1.0) (`self.CubeSize`)) (`self.ChunkLineElements`)))

(fn `UserConstructionScript`)