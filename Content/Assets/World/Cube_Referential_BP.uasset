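; Cube referential actor that supplies spawn parameters for voxels relative to its own placement in the world.
; SpawnVoxel converts a given location into a transform by subtracting the world origin, adding the actor's location and taking its rotation at unit scale.
; It also returns a uniform voxel size from CubeSize and the ChunkLineElements value, without spawning anything itself.
; The event graph and construction script are empty.
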(fn `SpawnVoxel`
  (params (location :type "Vector Structure"))
  (returns (transform :type "Transform Structure") (FVoxelSize :type "Vector Structure") (FChunkLineElements :type "IntVector Structure"))
  (bind (_returnvalue_x _returnvalue_y _returnvalue_z) (break `IntVector` (`GameplayStatics.GetWorldOriginLocation`)))
  (return (`KismetMathLibrary.MakeTransform` (+ (- location (`KismetMathLibrary.MakeVector` (`KismetMathLibrary.Conv_IntToDouble` _returnvalue_x) (`KismetMathLibrary.Conv_IntToDouble` _returnvalue_y) (`KismetMathLibrary.Conv_IntToDouble` _returnvalue_z))) (`self.K2_GetActorLocation`)) (`self.K2_GetActorRotation`)) (* (`KismetMathLibrary.MakeVector` 1.0 1.0 1.0) (`self.CubeSize`)) (`self.ChunkLineElements`)))

(fn `UserConstructionScript`)